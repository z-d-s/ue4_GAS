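; BP_Enemy is an enemy Blueprint that keeps an HP bar in sync with its health.
; On BeginPlay it binds to the attribute component's OnHpChanged delegate.
; Each change casts the HpBar widget component's user widget to WBP_EnemyHP and passes it the health-to-max ratio.
; Tick is empty, and an unconnected debug print of Health base and current values remains in the graph.
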(event Custom|OnHpChanged_Event
  (params (Health :type Float%20%28single-precision%29) (Maxhealth :type Float%20%28single-precision%29))
  (bind _aswbp_enemy_hp (Utilities|Casting|CastToWBP_EnemyHP (UserInterface|GetUserWidgetObject (Variables|Default|GetHpBar))))
  (Default|EvSetPercent _aswbp_enemy_hp (/ Health Maxhealth)))

(event EventBeginPlay
  (|CallParentFunction)
  (EventDispatchers|AssignOnHpChanged (Variables|Default|GetAttributeComp) (delegate Custom|OnHpChanged_Event)))

(event EventTick
  (params (DeltaSeconds :type Float%20%28single-precision%29)))

(fn ConstructionScript
  (|CallParentFunction))