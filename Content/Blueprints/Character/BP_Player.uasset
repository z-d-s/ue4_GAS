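; BP_Player is the player character Blueprint, which links health, mana and energy to the main HUD and handles death.
; Each attribute change event calls its parent, then sends the current/max ratio from AttributeComp to the matching ball widget in the GameInstance's MainUI.
; On death it calls the parent, starts the death montage and immediately disables input for player controller 0.
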(event EventBeginPlay
  (|CallParentFunction) ; This node is disabled and will not be called.\nDrag off pins to build functionality.
)

(event EventEvonMpChanged
  (params (Value :type Float%20%28single-precision%29) (MaxValue :type Float%20%28single-precision%29))
  (bind _attributecomp (Variables|Default|GetAttributeComp))
  (|CallParentFunction Value MaxValue)
  (Default|EvSetPercent (Variables|/Game/UMG/WBP_MainUI.WBP_MainUI_C|GetWBP_MPBall (Variables|/Game/Blueprints/BP_GameInstance.BP_GameInstance_C|GetMainUI (.AsBP%20Game%20Instance (Utilities|Casting|CastToBP_GameInstance (Game|GetGameInstance))))) (/ (.currentvalue (Variables|/Script/ue4_GAS.AttributeSetBase|GetMana _attributecomp)) (.currentvalue (Variables|/Script/ue4_GAS.AttributeSetBase|GetMaxMana _attributecomp)))))

(event EventEvonEnergyChanged
  (params (Value :type Float%20%28single-precision%29) (MaxValue :type Float%20%28single-precision%29))
  (bind _attributecomp (Variables|Default|GetAttributeComp))
  (|CallParentFunction Value MaxValue)
  (Default|EvSetPercent (Variables|/Game/UMG/WBP_MainUI.WBP_MainUI_C|GetWBP_EnergyBall (Variables|/Game/Blueprints/BP_GameInstance.BP_GameInstance_C|GetMainUI (.AsBP%20Game%20Instance (Utilities|Casting|CastToBP_GameInstance (Game|GetGameInstance))))) (/ (.currentvalue (Variables|/Script/ue4_GAS.AttributeSetBase|GetEnergy _attributecomp)) (.currentvalue (Variables|/Script/ue4_GAS.AttributeSetBase|GetMaxEnergy _attributecomp)))))

(event EventEvonHpChanged
  (params (Value :type Float%20%28single-precision%29) (MaxValue :type Float%20%28single-precision%29))
  (bind _attributecomp (Variables|Default|GetAttributeComp))
  (|CallParentFunction Value MaxValue)
  (Default|EvSetPercent (Variables|/Game/UMG/WBP_MainUI.WBP_MainUI_C|GetWBP_HPBall (Variables|/Game/Blueprints/BP_GameInstance.BP_GameInstance_C|GetMainUI (.AsBP%20Game%20Instance (Utilities|Casting|CastToBP_GameInstance (Game|GetGameInstance))))) (/ (.currentvalue (Variables|/Script/ue4_GAS.AttributeSetBase|GetHealth _attributecomp)) (.currentvalue (Variables|/Script/ue4_GAS.AttributeSetBase|GetMaxHealth _attributecomp)))))

(event EventEvonDeath
  (|CallParentFunction)
  (Animation|Montage|PlayMontage (Variables|Character|GetMesh) "/Game/Blueprints/AnimationBlueprints/Death_A_Montage.Death_A_Montage"
    (:then
      (Input|DisableInput (Game|GetPlayerController 0) 0))))

(fn ConstructionScript
  (|CallParentFunction))