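; Player controller that translates input into movement, look and combat actions on the controlled pawn.
; Movement axes follow the camera manager's forward and right vectors, and look axes add pitch and yaw input to the pawn.
; Jump casts the pawn to Character, while primary melee, health regen and dash cast to BP_CharacterBase and call its matching functions, leaving ability logic to the character.
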(event Input|ActionEvents|InputActionJump
  (params (Key :type Key%20Structure :default "None"))
  ;[1 1 1] Input
  (:Pressed
    (bind _ascharacter (Utilities|Casting|CastToCharacter (Pawn|GetControlledPawn)))
    (Character|Jump _ascharacter)))

(event Input|ActionEvents|InputActionPrimaryMelee
  (params (Key :type Key%20Structure :default "None"))
  ;[1 1 1] Primary Melee
  (:Pressed
    (bind _asbp_character_base (Utilities|Casting|CastToBP_CharacterBase (Pawn|GetControlledPawn)))
    (Default|MeleeAttack _asbp_character_base)))

(event Input|ActionEvents|InputActionHealthRegen
  (params (Key :type Key%20Structure :default "None"))
  ;[1 1 1] HealthRegen
  (:Pressed
    (bind _asbp_character_base (Utilities|Casting|CastToBP_CharacterBase (Pawn|GetControlledPawn)))
    (Default|HealthRegen _asbp_character_base)))

(event Input|ActionEvents|InputActionDash
  (params (Key :type Key%20Structure :default "None"))
  ;[1 1 1] Dash
  (:Pressed
    (bind _asbp_character_base (Utilities|Casting|CastToBP_CharacterBase (Pawn|GetControlledPawn)))
    (Default|Dash _asbp_character_base)))

(event Input|AxisEvents|InputAxisMoveForward
  (params (AxisValue :type Float%20%28single-precision%29))
  ;[1 1 1] Input
  (Pawn|Input|AddMovementInput (Pawn|GetControlledPawn) (Math|Vector|GetForwardVector (Camera|GetCameraRotation (Variables|Default|GetPlayerCameraManager))) AxisValue false))

(event Input|AxisEvents|InputAxisMoveRight
  (params (AxisValue :type Float%20%28single-precision%29))
  ;[1 1 1] Input
  (Pawn|Input|AddMovementInput (Pawn|GetControlledPawn) (Math|Vector|GetRightVector (Camera|GetCameraRotation (Variables|Default|GetPlayerCameraManager))) AxisValue false))

(event Input|AxisEvents|InputAxisLookUp
  (params (AxisValue :type Float%20%28single-precision%29))
  ;[1 1 1] Input
  (Pawn|Input|AddControllerPitchInput (Pawn|GetControlledPawn) AxisValue))

(event Input|AxisEvents|InputAxisLookRight
  (params (AxisValue :type Float%20%28single-precision%29))
  ;[1 1 1] Input
  (Pawn|Input|AddControllerYawInput (Pawn|GetControlledPawn) AxisValue))

(fn ConstructionScript)