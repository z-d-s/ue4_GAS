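; Base character Blueprint that uses the Gameplay Ability System for melee attacks and health regeneration.
; On BeginPlay it gets both abilities and binds to AttributeComp's HP, MP and energy changes; zero HP triggers death, while MP and energy handlers are empty.
; Weapon overlap with another character disables weapon collision and sends a melee damage gameplay event to itself with the victim as target, leaving damage to the ability side.
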(event OnComponentBeginOverlap(Weapon)
  (params (OverlappedComponent :type Primitive%20Component%20Object%20Reference) (OtherActor :type Actor%20Object%20Reference) (OtherComp :type Primitive%20Component%20Object%20Reference) (OtherBodyIndex :type Integer) (bFromSweep :type Boolean) (SweepResult :type Hit%20Result%20Structure%20%28by%20ref%29))
  ;[1 1 1] Overlap
  (if (and (Utilities|ClassIsChildOf (Utilities|GetClass OtherActor) "BP_CharacterBase_C") (!= OtherActor self))
    (CallFunction|ActiveWeaponCollision false)
    (Ability|SendGameplayEventtoActor self "(TagName=\"Skill.Ability.Melee_Damage\")" (Utilities|Struct|MakeGameplayEventData "(TagName=\"Skill.Ability.Melee_Damage\")" 0 OtherActor))))

(event Custom|MeleeAttack
  ;[1 1 1] Melee
  (Abilities|TryActivateAbilitybyClass (Variables|Default|GetAbilitySystemComp) "/Game/GAS/Melee/GA_Melee.GA_Melee_C" true))

(event Custom|Ev_OnDeath
  ;[1 1 1] OnDeath
  (Variables|Default|SetIsAlive false))

(event Custom|Ev_OnHpChanged
  (params (Value :type Float%20%28single-precision%29) (MaxValue :type Float%20%28single-precision%29))
  ;[1 1 1] BeginPlay
  (if (and (<= Value 0.0) (Variables|Default|GetIsAlive))
    (CallFunction|EvonDeath)))

(event Custom|HealthRegen
  ;[1 1 1] HealthRegen
  (Abilities|TryActivateAbilitybyClass (Variables|Default|GetAbilitySystemComp) "/Game/GAS/Health/GA_HealthRegen.GA_HealthRegen_C" true))

(event Custom|Ev_OnMpChanged
  (params (Value :type Float%20%28single-precision%29) (MaxValue :type Float%20%28single-precision%29))
  ;[1 1 1] BeginPlay
)

(event Custom|Ev_OnEnergyChanged
  (params (Value :type Float%20%28single-precision%29) (MaxValue :type Float%20%28single-precision%29))
  ;[1 1 1] BeginPlay
)

(event EventBeginPlay
  ;[1 1 1] BeginPlay
  (Variables|Default|SetIsAlive true)
  (CallFunction|GetGameAbilities)
  (EventDispatchers|AssignOnHpChanged (Variables|Default|GetAttributeComp) (delegate Custom|Ev_OnHpChanged))
  (EventDispatchers|BindEventtoOnMpChanged (Variables|Default|GetAttributeComp) (delegate Custom|Ev_OnMpChanged))
  (EventDispatchers|BindEventtoOnEnergyChanged (Variables|Default|GetAttributeComp) (delegate Custom|Ev_OnEnergyChanged)))

(fn ConstructionScript)

(fn ActiveWeaponCollision
  (params (Active :type Boolean))
  (if Active
    (Collision|SetCollisionEnabled (Variables|Default|GetWeapon) "QueryOnly")
    (else
      (Collision|SetCollisionEnabled (Variables|Default|GetWeapon) "NoCollision"))))

(fn GetGameAbilities
  (Class|CharacterBase|GetAbility "/Game/GAS/Melee/GA_Melee.GA_Melee_C")
  (Class|CharacterBase|GetAbility "/Game/GAS/Health/GA_HealthRegen.GA_HealthRegen_C"))