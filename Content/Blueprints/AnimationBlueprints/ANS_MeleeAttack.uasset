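; Anim notify state that opens the weapon hit window during melee attack animations.
; On begin it casts the mesh owner to BP_CharacterBase and turns weapon collision on through ActiveWeaponCollision.
; On end it turns that collision off, so the weapon collision is switched on only for the span of the notify.
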(fn ReceivedNotifyBegin
  (params (MeshComp :type Skeletal%20Mesh%20Component%20Object%20Reference) (Animation :type Anim%20Sequence%20Base%20Object%20Reference) (TotalDuration :type Float%20%28single-precision%29))
  (bind _asbp_character_base (Utilities|Casting|CastToBP_CharacterBase (Components|GetOwner MeshComp))
    (:then
      (Default|ActiveWeaponCollision _asbp_character_base true)
      (return true))
    (:CastFailed
      (return false))))

(fn ReceivedNotifyEnd
  (params (MeshComp :type Skeletal%20Mesh%20Component%20Object%20Reference) (Animation :type Anim%20Sequence%20Base%20Object%20Reference))
  (bind _asbp_character_base (Utilities|Casting|CastToBP_CharacterBase (Components|GetOwner MeshComp))
    (:then
      (Default|ActiveWeaponCollision _asbp_character_base false)
      (return true))
    (:CastFailed
      (return true))))