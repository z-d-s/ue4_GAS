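; BP_Enemy is an AI-controlled enemy that reacts to health changes and death on top of its parent class logic.
; Health changes push the current ratio into a WBP_EnemyHP widget on its HpBar component.
; On death it starts a death montage, stops the AI controller's brain logic, and destroys itself after a short delay.
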(event EventEvonHpChanged
  (params (Value :type Float%20%28single-precision%29) (MaxValue :type Float%20%28single-precision%29))
  (|CallParentFunction Value MaxValue)
  (bind _aswbp_enemy_hp (Utilities|Casting|CastToWBP_EnemyHP (UserInterface|GetUserWidgetObject (Variables|Default|GetHpBar))))
  (Default|EvSetPercent _aswbp_enemy_hp (/ Value MaxValue)))

(event EventEvonDeath
  (|CallParentFunction)
  (Animation|Montage|PlayMontage (Variables|Character|GetMesh) "/Game/Blueprints/AnimationBlueprints/Death_A_Montage.Death_A_Montage"
    (:then
      (CallFunction|StopControllerLogic)
      (Utilities|FlowControl|Delay 1.6)
      (Actor|DestroyActor))))

(fn ConstructionScript
  (|CallParentFunction))

(fn StopControllerLogic
  (bind _asaicontroller (Utilities|Casting|CastToAIController (Pawn|GetController)))
  (AI|Logic|StopLogic (Variables|/Script/AIModule.AIController|GetBrainComponent _asaicontroller) "Death"))