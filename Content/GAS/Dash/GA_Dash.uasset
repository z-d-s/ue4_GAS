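; GA_Dash is a gameplay ability that launches the owning character forward and damages targets along the way.
; On activation it commits, zeroes ground friction, applies a forward velocity-change impulse, sets pawn collision to overlap and plays the dash montage.
; While active, a Skill.Dash.DealDamage gameplay event applies GE_Dash_Damage to its payload target.
; When the montage ends or is interrupted, friction and pawn blocking are restored and the ability ends.
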(event Ability|EventActivateAbility
  (Ability|CommitAbility)
  (bind _ascharacter (Utilities|Casting|CastToCharacter (Ability|GetOwningActorfromActorInfo))
    (:then
      (Variables|Default|SetOriGroundFriction (Variables|/Script/Engine.CharacterMovementComponent|GetGroundFriction (Variables|/Script/Engine.Character|GetCharacterMovement _ascharacter)))
      (Variables|/Script/Engine.CharacterMovementComponent|SetGroundFriction (Variables|/Script/Engine.Character|GetCharacterMovement _ascharacter) 0.0)
      (Physics|AddImpulse (Variables|/Script/Engine.Character|GetCharacterMovement _ascharacter) (* (Transformation|GetActorForwardVector _ascharacter) 1.5e+03) true)
      (bind _characterbase (CallFunction|GetPlayerCharacterandController))
      (Default|SetCollisiontoPawn _characterbase "ECR_Overlap")
      (|PlayMontageandWaitProxy "None" "/Game/Blueprints/AnimationBlueprints/Ability_Dash_Montage.Ability_Dash_Montage" 1.0 "None" true 1.0 0.0
        (:then
          (bind _payload (Ability|Tasks|WaitGameplayEvent "(TagName=\"Skill.Dash.DealDamage\")" 0)
            (:EventReceived
              (GameplayEffects|ApplyGameplayEffectToTarget (Ability|TargetData|AbilityTargetDatafromActor (.Target (Utilities|Struct|BreakGameplayEventData _payload))) "/Game/GAS/Dash/GE_Dash_Damage.GE_Dash_Damage_C" 1 1))))
        (:OnCompleted
          (Variables|/Script/Engine.CharacterMovementComponent|SetGroundFriction (Variables|/Script/Engine.Character|GetCharacterMovement _ascharacter) (Variables|Default|GetOriGroundFriction) :!label _label)
          (bind _characterbase_2 (CallFunction|GetPlayerCharacterandController))
          (Default|SetCollisiontoPawn _characterbase_2 "ECR_Block")
          (Ability|EndAbility))
        (:OnBlendOut
          (goto _label))
        (:OnInterrupted
          (goto _label))
        (:OnCancelled
          (goto _label))))
    (:CastFailed
      (Ability|EndAbility))))

(event Ability|EventOnEndAbility
  (params (bWasCancelled :type Boolean)))